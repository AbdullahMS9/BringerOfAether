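; Heal is a player effect Blueprint for a turn-based battle that restores health to the character who uses it.
; On activation it attaches a scaled steam particle emitter to a new component on the source character, then adds EffectAmount to that character's Health.
; It then casts the game mode to BattleGameMode and switches player turns; the target serves only as context for fetching that game mode.
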(event EventOnActivated
  (params (sourceCharacter :type Player%20Character%20Object%20Reference) (targetCharacter :type Player%20Character%20Object%20Reference))
  (CallFunction|CreateVisualEffects sourceCharacter targetCharacter)
  (CallFunction|UpdatePlayerStats sourceCharacter targetCharacter)
  (bind _asbattle_game_mode (Utilities|Casting|CastToBattleGameMode (Game|GetGameMode targetCharacter)))
  (Default|SwitchPlayerTurns _asbattle_game_mode))

(fn CreateVisualEffects
  (params (SourcePlayer :type Player%20Character%20Object%20Reference) (TargetPlayer :type Player%20Character%20Object%20Reference))
  (bind _returnvalue (Game|AddComponentbyClass SourcePlayer 0 "/Script/Engine.ParticleSystemComponent"))
  (Effects|SpawnEmitterAttached "/Game/StarterContent/Particles/P_Steam_Lit.P_Steam_Lit" _returnvalue "None" "0, 0, 0" "0, 0, 0" "2.000000,2.000000,2.000000"))

(fn UpdatePlayerStats
  (params (SourcePlayer :type Player%20Character%20Object%20Reference) (TargetPlayer :type Player%20Character%20Object%20Reference))
  (Variables|/Script/BringerOfAether.PlayerCharacter|Sethealth SourcePlayer (+ (Variables|Default|GeteffectAmount) (Variables|/Script/BringerOfAether.PlayerCharacter|Gethealth SourcePlayer))))