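; DoubleSidedExplosion is a turn-based battle effect that damages the opponent at the cost of recoil to its user.
; On activation it spawns an explosion on the target, deducts magic and target health, and prints the result.
; Recoil is a fixed, unclamped health loss.
; It switches turns through MainGameMode, then destroys the target and ends the battle if its health is zero; the user's death is not checked.
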(event EventOnActivated
  (params (activator :type Actor%20Stats%20Component%20Object%20Reference) (other :type Actor%20Stats%20Component%20Object%20Reference))
  (bind _returnvalue (Components|GetOwner other))
  (CallFunction|Animate activator other)
  (CallFunction|CreateVisualEffects (Components|GetOwner activator) _returnvalue)
  (CallFunction|UpdateStats activator other)
  (bind _asmain_game_mode (Utilities|Casting|CastToMainGameMode (Game|GetGameMode _returnvalue)))
  (Default|SwitchTurns _asmain_game_mode)
  (if (== 0.0 (Variables|/Script/BringerOfAether.ActorStatsComponent|Gethealth other))
    (Actor|DestroyActor _returnvalue)
    (Default|EndBattle _asmain_game_mode)))

(fn CreateVisualEffects
  (params (Activator :type Actor%20Object%20Reference) (Other :type Actor%20Object%20Reference))
  (Effects|SpawnEmitteratLocation Other "/Game/StarterContent/Particles/P_Explosion.P_Explosion" (Transformation|GetActorLocation Other) "0, 0, 0" "2.000000,2.000000,2.000000"))

(fn Animate
  (params (Activator :type Actor%20Stats%20Component%20Object%20Reference) (Other :type Actor%20Stats%20Component%20Object%20Reference)))

(fn UpdateStats
  (params (Activator :type Actor%20Stats%20Component%20Object%20Reference) (Other :type Actor%20Stats%20Component%20Object%20Reference))
  (bind _effectamount (Variables|Default|GeteffectAmount))
  (Variables|/Script/BringerOfAether.ActorStatsComponent|Sethealth Activator (- (Variables|/Script/BringerOfAether.ActorStatsComponent|Gethealth Activator) 1e+01))
  (Variables|/Script/BringerOfAether.ActorStatsComponent|Setmagic Activator (Math|Float|Clamp(Float) (- (Variables|/Script/BringerOfAether.ActorStatsComponent|Getmagic Activator) (Variables|Default|GeteffectCost)) 0.0 1e+02))
  (Variables|/Script/BringerOfAether.ActorStatsComponent|Sethealth Other (Math|Float|Clamp(Float) (- (Variables|/Script/BringerOfAether.ActorStatsComponent|Gethealth Other) _effectamount) 0.0 1e+02))
  (Development|PrintString 0 (Utilities|String|Append (Utilities|String|Append "Double Sided Explosion dealt " (Utilities|String|ToString(Float) _effectamount)) " damage! 
You took 10 damage from the recoil!") true true "(R=0.838542,G=0.182653,B=0.000000,A=1.000000)" 3.0))