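; WeakExplosion is a player effect for turn-based battles that damages the target with an explosion at the cost of the activator's Magic.
; On activation it spawns an explosion emitter on the target's owner and subtracts level-scaled damage from Health, clamping both stats.
; It then shows the damage in the MainGameMode HUD battle text and switches turns.
; The Animate step is an empty stub.
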(event EventOnActivated
  (params (activator :type Actor%20Stats%20Component%20Object%20Reference) (other :type Actor%20Stats%20Component%20Object%20Reference))
  (bind _returnvalue (Components|GetOwner other))
  (CallFunction|Animate activator other)
  (CallFunction|CreateVisualEffects (Components|GetOwner activator) _returnvalue)
  (CallFunction|UpdateStats activator other)
  (bind _asmain_game_mode (Utilities|Casting|CastToMainGameMode (Game|GetGameMode _returnvalue)))
  (Rendering|Components|TextRender|SetText (Variables|/Game/Blueprints/UI/HUD.HUD_C|GetBattleText (Variables|/Game/Blueprints/GameModes/MainGameMode.MainGameMode_C|GetHUD _asmain_game_mode)) (Utilities|Text|ToText(String) (Utilities|String|Append (Utilities|String|Append "Explosion dealt " (Utilities|String|ToString(Float) (* (Variables|Default|GeteffectAmount) (+ (* (Variables|/Script/BringerOfAether.ActorStatsComponent|Getlevel activator) 0.1) 1.0)))) " damage!")))
  (Default|SwitchTurns _asmain_game_mode))

(fn CreateVisualEffects
  (params (Activator :type Actor%20Object%20Reference) (Other :type Actor%20Object%20Reference))
  (Effects|SpawnEmitteratLocation Other "/Game/StarterContent/Particles/P_Explosion.P_Explosion" (Transformation|GetActorLocation Other) "0, 0, 0" "2.000000,2.000000,2.000000"))

(fn Animate
  (params (Activator :type Actor%20Stats%20Component%20Object%20Reference) (Other :type Actor%20Stats%20Component%20Object%20Reference)))

(fn UpdateStats
  (params (Activator :type Actor%20Stats%20Component%20Object%20Reference) (Other :type Actor%20Stats%20Component%20Object%20Reference))
  (Variables|/Script/BringerOfAether.ActorStatsComponent|Setmagic Activator (Math|Float|Clamp(Float) (- (Variables|/Script/BringerOfAether.ActorStatsComponent|Getmagic Activator) (Variables|Default|GeteffectCost)) 0.0 1e+02))
  (Variables|/Script/BringerOfAether.ActorStatsComponent|Sethealth Other (Math|Float|Clamp(Float) (- (Variables|/Script/BringerOfAether.ActorStatsComponent|Gethealth Other) (* (Variables|Default|GeteffectAmount) (+ (* (Variables|/Script/BringerOfAether.ActorStatsComponent|Getlevel Activator) 0.1) 1.0))) 0.0 1e+02)))