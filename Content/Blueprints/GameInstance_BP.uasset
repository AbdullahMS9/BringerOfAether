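; Game Instance that records defeated enemy IDs and handles level switching with player placement.
; KillEnemy adds the given ID to the Defeated collection.
; SwitchLevel stores the pawn's transform, control rotation and actor rotation, opens the named level, then reapplies them after a short fixed delay.
; Hard-coded relative transform and rotation calls follow the restores, overwriting the restored actor transform and rotation.
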(event Custom|SwitchLevel
  (params (Level%20Name :type Name))
  (bind _returnvalue (Game|Player|GetPlayerPawn 0))
  (bind _returnvalue_2 (Game|GetPlayerCharacter 0))
  (Variables|Default|SetStoredTransform (Transformation|GetActorTransform _returnvalue))
  (Variables|Default|SetStoredRotation (Pawn|GetControlRotation _returnvalue :!class /Script/Engine.Pawn))
  (Variables|Default|SetStoredRotation2 (Transformation|GetActorRotation _returnvalue))
  (Game|OpenLevel(byName) Level%20Name)
  (Utilities|FlowControl|Delay 0.2)
  (Transformation|SetActorTransform (Game|Player|GetPlayerPawn 0) (Variables|Default|GetStoredTransform))
  (Transformation|SetActorRelativeTransform (Game|Player|GetPlayerPawn 0) (Math|Transform|MakeTransform "0, 0,600.000000") false false)
  (Pawn|SetControlRotation (Pawn|GetController _returnvalue_2) (Variables|Default|GetStoredRotation))
  (Transformation|SetActorRotation _returnvalue_2 (Variables|Default|GetStoredRotation2))
  (Transformation|SetActorRelativeRotation _returnvalue_2 "0,180.000000, 0"))

(event Custom|Kill%20Enemy
  (params (EnemyID :type Name))
  (Utilities|Array|Add (Variables|Default|GetDefeated) EnemyID))