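; Game mode that runs turn-based battles between the player and an opponent and creates the HUD at BeginPlay.
; StartBattle disables player input, moves the pawn to the opponent's battle location facing it, and shows the battle UI and cursor.
; SwitchTurns alternates the acting ActorStatsComponent, showing effect choices only on the player's turn.
; On its turn the opponent waits briefly, then constructs and activates a random effect class against the player.
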(event Custom|OnOpponentTurn
  (bind _opponentstats (Variables|Default|GetOpponentStats))
  (Utilities|FlowControl|Delay (Math|Random|RandomFloatinRange 0.5 2.0))
  (bind _returnvalue (Game|ConstructObjectfromClass (.OutItem (Utilities|Array|Random (Variables|/Script/BringerOfAether.ActorStatsComponent|GetplayerEffects _opponentstats))) _opponentstats))
  (Class|PlayerEffect|OnActivated _returnvalue _opponentstats (Actor|GetComponentbyClass (Game|Player|GetPlayerPawn 0) "/Script/BringerOfAether.ActorStatsComponent")))

(event EventBeginPlay
  (bind _returnvalue (UserInterface|CreateWidget "/Game/Blueprints/UI/HUD.HUD_C" (Game|GetPlayerController 0)))
  (bind _output_get (Variables|Default|SetHUD _returnvalue))
  (Variables|Default|SetCurrentActorTurn (Actor|GetComponentbyClass (Game|Player|GetPlayerPawn 0) "/Script/BringerOfAether.ActorStatsComponent"))
  (Widget|SetVisibility (Variables|/Game/Blueprints/UI/HUD.HUD_C|GetBattleUI _output_get) "Hidden")
  (UserInterface|Viewport|AddtoViewport _output_get 0))

(event EventTick
  (params (DeltaSeconds :type Float%20%28single-precision%29)))

(fn ConstructionScript)

(fn StartBattle
  (params (Opponent%20Stats :type Actor%20Stats%20Component%20Object%20Reference))
  (bind _returnvalue (Game|Player|GetPlayerPawn 0))
  (bind _returnvalue_2 (Game|GetPlayerController 0))
  (bind _hud (Variables|Default|GetHUD))
  (bind _output_get (Variables|Default|SetOpponentStats Opponent%20Stats))
  (Input|DisableInput _returnvalue 0)
  (Transformation|SetActorLocation _returnvalue (Transformation|GetWorldLocation (Actor|GetComponentbyClass (Components|GetOwner _output_get) "/Game/Blueprints/PlayerCharacters/PlayerBattleLocation.PlayerBattleLocation_C")) false false)
  (Pawn|SetControlRotation _returnvalue_2 (Math|Rotator|FindLookatRotation (Transformation|GetActorLocation _returnvalue) (Transformation|GetActorLocation (Components|GetOwner _output_get))))
  (Variables|/Script/Engine.PlayerController|SetbShowMouseCursor _returnvalue_2 true)
  (Widget|SetVisibility (Variables|/Game/Blueprints/UI/HUD.HUD_C|GetBattleUI _hud) "Visible")
  (Default|OnRefresh (Variables|/Game/Blueprints/UI/HUD.HUD_C|GetPlayerEffectsDisplay _hud)))

(fn SwitchTurns
  (bind _returnvalue (Game|Player|GetPlayerPawn 0))
  (bind _hud (Variables|Default|GetHUD))
  (bind _returnvalue_2 (Actor|GetComponentbyClass _returnvalue "/Script/BringerOfAether.ActorStatsComponent"))
  (bind _playereffectsdisplay (Variables|/Game/Blueprints/UI/HUD.HUD_C|GetPlayerEffectsDisplay _hud))
  (if (== (Variables|Default|GetCurrentActorTurn) _returnvalue_2)
    (Variables|Default|SetCurrentActorTurn (Variables|Default|GetOpponentStats))
    (Widget|SetVisibility _playereffectsdisplay "Hidden")
    (CallFunction|OnOpponentTurn)
    (else
      (Variables|Default|SetCurrentActorTurn _returnvalue_2)
      (Widget|SetVisibility _playereffectsdisplay "Visible"))))

(fn EndBattle
  (Widget|SetVisibility (Variables|/Game/Blueprints/UI/HUD.HUD_C|GetBattleUI (Variables|Default|GetHUD)) "Hidden")
  (Input|EnableInput (Game|Player|GetPlayerPawn 0) 0))