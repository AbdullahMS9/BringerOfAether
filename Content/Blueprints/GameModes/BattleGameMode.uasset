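; BattleGameMode is the game mode for a two-player, turn-based battle, tracking whose turn it is.
; On BeginPlay it assigns placed PlayerCharacters to Player1 or Player2 by their IsMainPlayer flag, creates the HUD for the first player controller and gives Player1 the first turn.
; SwitchPlayerTurns flips CurrentTurnPlayer and calls UpdateHUD, which shows only the active player's button group.
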(event Custom|UpdateHUD
  (if (== (Variables|Default|GetCurrentTurnPlayer) (Variables|Default|GetPlayer1))
    (Widget|SetVisibility (Variables|/Game/Blueprints/UI/HUD.HUD_C|GetPlayer2ButtonGroup (Variables|Default|GetHUD)) "Hidden")
    (Widget|SetVisibility (Variables|/Game/Blueprints/UI/HUD.HUD_C|GetPlayer1ButtonGroup (Variables|Default|GetHUD)) "Visible")
    (else
      (Widget|SetVisibility (Variables|/Game/Blueprints/UI/HUD.HUD_C|GetPlayer1ButtonGroup (Variables|Default|GetHUD)) "Hidden")
      (Widget|SetVisibility (Variables|/Game/Blueprints/UI/HUD.HUD_C|GetPlayer2ButtonGroup (Variables|Default|GetHUD)) "Visible"))))

(event EventBeginPlay
  (bind _outactors (Actor|GetAllActorsOfClass "/Script/BringerOfAether.PlayerCharacter"))
  (for _array_element _outactors
    (if (Variables|/Script/BringerOfAether.PlayerCharacter|GetisMainPlayer _array_element)
      (Variables|Default|SetPlayer1 _array_element)
      (else
        (Variables|Default|SetPlayer2 _array_element))))
  (bind _returnvalue (UserInterface|CreateWidget "/Game/Blueprints/UI/HUD.HUD_C" (Game|GetPlayerController 0)))
  (bind _output_get (Variables|Default|SetHUD _returnvalue))
  (UserInterface|Viewport|AddtoViewport _output_get 0)
  (Variables|Default|SetCurrentTurnPlayer (Variables|Default|GetPlayer1))
  (CallFunction|UpdateHUD))

(fn ConstructionScript)

(fn SwitchPlayerTurns
  (if (== (Variables|Default|GetCurrentTurnPlayer) (Variables|Default|GetPlayer1))
    (Variables|Default|SetCurrentTurnPlayer (Variables|Default|GetPlayer2))
    (else
      (Variables|Default|SetCurrentTurnPlayer (Variables|Default|GetPlayer1))))
  (CallFunction|UpdateHUD))